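; BP_Level_Base is a level base Blueprint that manages selection among MovableObject actors and totals their points when the level ends.
; On BeginPlay it enables player input, gathers every MovableObject, and passes the selected one to a component that sends it a select message.
; The change-selection event deselects the current object and cycles to the next, wrapping around.
; The end-level event has each object count its points, then accumulates them.
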(event `self.ReceiveBeginPlay`
  (bind _outactors (`GameplayStatics.GetAllActorsOfClass` "/Game/Gameplay/Objets/MovableObject.MovableObject_C"))
  (bind _output_get (set `self.AllObjectsSelectable` _outactors))
  (`self.EnableInput` (`GameplayStatics.GetPlayerController` 0))
  (bind _output_get_2 (set `self.ActualObjectSelected` (`|GetArrayItem` _output_get (`self.Index`)) :!label _label))
  (bind _output_get_3 (set `/Game/Gameplay/Levels/C_ActualObjectSelected.objectSelected` _output_get_2 (`self.C_ActualObjectSelected`)))
  (message `/Game/Gameplay/Interface/IActorSelected.SelectMyActor` _output_get_3))

(event `EventChangeObjectSelected_Event`
  (bind _index (`self.Index`))
  (if (< (+ (`KismetArrayLibrary.Array_Length` (`self.AllObjectsSelectable`)) -2) _index)
    (set `self.Index` 0)
    (else
      (set `self.Index` (+ _index 1))))
  (message `/Game/Gameplay/Interface/IActorSelected.DiselectMyActor` (`self.ActualObjectSelected`))
  (goto _label))

(event `EventEndLevel_Event`
  (for _array_element (`self.AllObjectsSelectable`)
    (bind _asmovable_object (cast `/Game/Gameplay/Objets/MovableObject` _array_element))
    (`/Game/Gameplay/Objets/MovableObject.EventCountPoints_Event` _asmovable_object)
    (set `self.acumulatePoints` (+ (`self.acumulatePoints`) (`/Game/Gameplay/Objets/MovableObject.points` _asmovable_object)))))

(fn `UserConstructionScript`)